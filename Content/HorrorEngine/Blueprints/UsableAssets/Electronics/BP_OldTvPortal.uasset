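; BP_OldTvPortal is an old TV that opens a portal, extending a parent's portal-opening logic.
; Portal Opening calls the parent, spawns a Portal actor at the TV's location and prints a debug string.
; BeginLoad eases the Portal0 component over two seconds to a point just above the player's position, computed relative to the TV.
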(event `/Game/HorrorEngine/Blueprints/Core/HorrorEngineInterface.BeginLoad`
  (bind _returnvalue_location (`KismetMathLibrary.BreakTransform` (`KismetMathLibrary.MakeRelativeTransform` (`self.GetTransform` (`GameplayStatics.GetPlayerCharacter` 0)) (`SceneComponent.K2_GetComponentToWorld` (`self.Tv`)))))
  (`KismetSystemLibrary.MoveComponentTo` (`self.Portal_0`) (+ _returnvalue_location (0.0 0.0 50.0)) (struct) false true 2.0 true))

(fn `Portal Opening`
  (`parent.Portal Opening`)
  (`|SpawnActorFromClass` "/Game/HorrorEngine/Blueprints/UsableAssets/PortalAndTriggers/Portal.Portal_C" (`KismetMathLibrary.Conv_VectorToTransform` (`SceneComponent.K2_GetComponentLocation` (`self.Tv`))) "AlwaysSpawn" "MultiplyWithRoot" null null)
  (`KismetSystemLibrary.PrintString` "PORTAL OPENING"))

(fn `UserConstructionScript`
  (`parent.UserConstructionScript`))