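; One-shot overlap trigger that sends the monster to investigate a set position when the player pawn enters it.
; The construction script caches a BP_Enemy from the level as Monster.
; On player overlap it passes InvestigatePosition via TriggerGiveInvestigPosMessage, then destroys itself and prints a debug string.
; An Italian author note suggests placing it away from the player and teleporting it onto them with a horror event.
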(event `self.OverlapTrigger.OnComponentBeginOverlap`
  (params (OverlappedComponent :type "PrimitiveComponent Object Reference") (OtherActor :type "Actor Object Reference") (OtherComp :type "PrimitiveComponent Object Reference") (OtherBodyIndex :type Integer) (bFromSweep :type Boolean) (SweepResult :type "HitResult Structure (by ref)"))
  ;[1 1 1] CONSIGLIO: TENERLO IN UNA ZONA LONTANA DAL PLAYER E METTERE UN HORROR EVENT PER TELETRASPORTARE IL TRIGGER SUL PLAYER
  (if (== OtherActor (`GameplayStatics.GetPlayerPawn` 0))
    (message `/Game/LoryTest/Blueprints/Interface/MonsterTriggers.TriggerGiveInvestigPos` (`self.Monster`) (`self.InvestigatePosition`))
    (`self.K2_DestroyActor`)
    (`KismetSystemLibrary.PrintString` "Hello")))

(fn `UserConstructionScript`
  (bind _returnvalue (`GameplayStatics.GetActorOfClass` "/Game/LoryTest/Blueprints/BP_Enemy.BP_Enemy_C"))
  (set `self.Monster` _returnvalue))