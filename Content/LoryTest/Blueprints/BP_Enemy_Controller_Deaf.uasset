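; AI controller for the "Deaf" enemy, which, despite the name, reacts only to hearing stimuli.
; On BeginPlay it caches the HorrorEngine player character and runs its behavior tree.
; Heard stimuli write their location to the InvestigatePos blackboard key and message the pawn, while HandleTouchSense is an empty stub.
; UpdateNearDoor feeds door state to the blackboard, writing IsDoorLocked into the IsDoorOpen key.
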(event `self.ReceiveBeginPlay`
  (bind _ashorror_engine_character (cast `/Game/HorrorEngine/Blueprints/Core/HorrorEngineCharacter` (`GameplayStatics.GetPlayerCharacter` 0))
    (:`then`
      (set `self.PlayerReference` _ashorror_engine_character)
      (`self.RunBehaviorTree` (`self.BehaviourTree`)))
    (:`CastFailed`
      (`KismetSystemLibrary.PrintString` "Cannot find player"))))

(event `self.Update Near Door`
  (params (NearDoor :type Boolean) (IsDoorLocked :type Boolean))
  (bind _blackboard (`self.Blackboard`))
  ;[1 1 1] Near Door Update
  (bind _output_get (set `self.NearDoor` NearDoor))
  (`BlackboardComponent.SetValueAsBool` _blackboard "NearDoor" _output_get)
  (`BlackboardComponent.SetValueAsBool` _blackboard "IsDoorOpen" IsDoorLocked))

(event `self.AIPerception.OnTargetPerceptionUpdated`
  (params (Actor :type "Actor Object Reference") (Stimulus :type "AIStimulus Structure"))
  (`self.HandleHearSense` Stimulus Actor))

(event `self.AIPerception.OnPerceptionUpdated`
  (params (UpdatedActors :type "Array of Actor Object Reference (by ref)")))

(event `self.AIPerception.OnTargetPerceptionInfoUpdated`
  (params (UpdateInfo :type "ActorPerceptionUpdateInfo Structure (by ref)")))

(fn `HandleHearSense`
  (params (Stimulus :type "AIStimulus Structure") (Monster :type "Actor Object Reference"))
  (bind _returnvalue (`AIPerceptionSystem.GetSenseClassForStimulus` Stimulus))
  (if (== _returnvalue "/Script/AIModule.AISense_Hearing")
    (`BlackboardComponent.SetValueAsVector` (`self.Blackboard`) "InvestigatePos" (`.StimulusLocation` (break `AIStimulus` Stimulus)))
    (message `/Game/LoryTest/Blueprints/Interface/MonsterInterface.ActionOnHearingSomething` (`self.K2_GetPawn`))
    (else
      (return))))

(fn `HandleTouchSense`)

(fn `UserConstructionScript`)