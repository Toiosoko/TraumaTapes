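; Enemy for a horror game that senses, chases and attacks the player, with its state fed to an AI controller and blackboard.
; Pawn sensing sets the seen and last-known position keys, and a retriggerable delay flips chasing to investigating once sightings stop.
; Hits briefly flag player contact the same way, while door events report nearby doors and lock state to the controller.
; Attack deals heavy damage, then signals its end; SmashDoor is empty.
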(event `self.PawnSensing.OnSeePawn`
  (params (Pawn :type "Pawn Object Reference"))
  (bind _returnvalue (`AIBlueprintHelperLibrary.GetBlackboard` (`AIBlueprintHelperLibrary.GetAIController` self)))
  ;[1 1 1] Chase Player
  (bind _ashorror_engine_character (cast `/Game/HorrorEngine/Blueprints/Core/HorrorEngineCharacter` Pawn))
  (`|ExecutionSequence`
    (:`then_0`
      (`BlackboardComponent.SetValueAsBool` _returnvalue "SeeingPlayer" true)
      (`BlackboardComponent.SetValueAsBool` _returnvalue "Investigating" false)
      (`BlackboardComponent.SetValueAsVector` _returnvalue "InvestigatePos" (`self.K2_GetActorLocation` _ashorror_engine_character)))
    (:`then_1`
      (`KismetSystemLibrary.RetriggerableDelay` 0.6)
      (`BlackboardComponent.SetValueAsBool` _returnvalue "SeeingPlayer" false)
      (`BlackboardComponent.SetValueAsBool` _returnvalue "Investigating" true))))

(event `UpdateLocalDoor`
  (params (Door :type "/Game/LoryTest/Blueprints/DoorPhysNew Object Reference"))
  (bind _output_get (set `self.DoorNear` Door))
  (message `/Game/LoryTest/Blueprints/Interface/IF_DoorNear.Update Near Door` (`AIBlueprintHelperLibrary.GetAIController` self) true (`/Game/LoryTest/Blueprints/DoorPhysNew.IsLocked` _output_get)))

(event `SmashDoor`)

(event `ClearDoor`
  (set `self.DoorNear` null)
  (message `/Game/LoryTest/Blueprints/Interface/IF_DoorNear.Update Near Door` (`AIBlueprintHelperLibrary.GetAIController` self) false false))

(event `self.ReceiveHit`
  (params (MyComp :type "PrimitiveComponent Object Reference") (Other :type "Actor Object Reference") (OtherComp :type "PrimitiveComponent Object Reference") (bSelfMoved :type Boolean) (HitLocation :type "Vector Structure") (HitNormal :type "Vector Structure") (NormalImpulse :type "Vector Structure") (Hit :type "HitResult Structure (by ref)"))
  (bind _returnvalue (`AIBlueprintHelperLibrary.GetBlackboard` (`AIBlueprintHelperLibrary.GetAIController` self)))
  (if (== Other (`GameplayStatics.GetPlayerCharacter` 0))
    (`|ExecutionSequence`
      (:`then_0`
        (`BlackboardComponent.SetValueAsBool` _returnvalue "IsTouchingPlayer" true))
      (:`then_1`
        (`KismetSystemLibrary.RetriggerableDelay` 0.5)
        (`BlackboardComponent.SetValueAsBool` _returnvalue "IsTouchingPlayer" false)))))

(event `Attack`
  (bind _asmaster (`/Game/HorrorEngine/Blueprints/Core/HorrorEngineFunctions.GetPlayer`))
  (`/Game/HorrorEngine/HorrorEngine.GetDamage` :`self` _asmaster :`DamagePoint` 100.0)
  (`self.OnAttackEnd`))

(fn `UserConstructionScript`)