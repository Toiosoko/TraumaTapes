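; AI controller for the Stalker enemy that turns sight perception of the player into Blackboard data.
; HandleSightSense sets TargetObject while the player is seen and, when sight is lost, clears it and stores LastKnownLocation.
; It calls ToggleConeMessage with true on the player in both cases.
; On sight loss it also tries to clear ChasePlayer, but casts the sensed player, rather than the controlled pawn, to BP_Enemy_Stalker.
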(fn `HandleSightSense`
  (params (Actor :type "Actor Object Reference") (Stimulus :type "AIStimulus Structure"))
  (bind (_age _expirationage _strength _stimuluslocation _receiverlocation _tag _bsuccessfullysensed) (break `AIStimulus` Stimulus))
  (bind _returnvalue (`GameplayStatics.GetPlayerCharacter` 0))
  (bind _returnvalue_2 (`AIPerceptionSystem.GetSenseClassForStimulus` Stimulus))
  (if (== _returnvalue_2 "/Script/AIModule.AISense_Sight")
    (if (== Actor _returnvalue)
      (`BlackboardComponent.SetValueAsObject` (`self.Blackboard`) "TargetObject" (`KismetMathLibrary.SelectObject` (`GameplayStatics.GetPlayerCharacter` 0) null _bsuccessfullysensed))
      (message `/Game/LoryTest/Blueprints/Interface/PlayerInterface.ToggleCone` _returnvalue true)
      (if (not _bsuccessfullysensed)
        (`BlackboardComponent.SetValueAsVector` (`self.Blackboard`) "LastKnownLocation" _stimuluslocation)
        (message `/Game/LoryTest/Blueprints/Interface/PlayerInterface.ToggleCone` _returnvalue true)
        (bind _asbp_enemy_stalker (cast `/Game/LoryTest/Blueprints/BP_Enemy_Stalker` Actor))
        (set `/Game/LoryTest/Blueprints/BP_Enemy_Stalker.ChasePlayer` false _asbp_enemy_stalker))
      (else
        (return)))
    (else
      (return))))

(fn `UserConstructionScript`
  (`parent.UserConstructionScript`))