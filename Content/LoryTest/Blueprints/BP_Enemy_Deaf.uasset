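; BP_Enemy_Deaf is a child enemy Blueprint that detects the player by proximity, with the inherited vision cone's collision disabled.
; Overlapping CheckPlayerDistance sets the player as the AI blackboard's TargetObject and starts running; leaving clears it and returns to walking.
; Hearing events also start running, and reaching the destination returns to walking.
; Save events cache state on the player's save component and restore it, re-triggering the investigate position.
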(event `self.CheckPlayerDistance.OnComponentBeginOverlap`
  (params (OverlappedComponent :type "PrimitiveComponent Object Reference") (OtherActor :type "Actor Object Reference") (OtherComp :type "PrimitiveComponent Object Reference") (OtherBodyIndex :type Integer) (bFromSweep :type Boolean) (SweepResult :type "HitResult Structure (by ref)"))
  (bind _returnvalue (`GameplayStatics.GetPlayerCharacter` 0))
  (if (== OtherActor _returnvalue)
    (`BlackboardComponent.SetValueAsObject` (`AIBlueprintHelperLibrary.GetBlackboard` (`AIBlueprintHelperLibrary.GetAIController` self)) "TargetObject" _returnvalue)
    (if (not (`self.IsRunning`))
      (`self.Toggle Walk/Run`))))

(event `self.CheckPlayerDistance.OnComponentEndOverlap`
  (params (OverlappedComponent :type "PrimitiveComponent Object Reference") (OtherActor :type "Actor Object Reference") (OtherComp :type "PrimitiveComponent Object Reference") (OtherBodyIndex :type Integer))
  (if (== OtherActor (`GameplayStatics.GetPlayerCharacter` 0))
    (`BlackboardComponent.SetValueAsObject` (`AIBlueprintHelperLibrary.GetBlackboard` (`AIBlueprintHelperLibrary.GetAIController` self)) "TargetObject" null)
    (if (`self.IsRunning`)
      (`self.Toggle Walk/Run`))))

(event `/Game/HorrorEngine/Blueprints/Core/HorrorEngineInterface.CollectSaveData`
  ;[0 1 0.5572] Save Settings
  (bind _asmaster (`/Game/HorrorEngine/Blueprints/Core/HorrorEngineFunctions.GetPlayer`))
  (`KismetArrayLibrary.Array_Add` (`/Game/HorrorEngine/Blueprints/Core/HE_SaveGameComponent.AssetCache` (`/Game/HorrorEngine/HorrorEngine.HE_SaveGameComponent` _asmaster)) (make `/Game/HorrorEngine/Blueprints/Structures/SaveStructures/AssetsSave` (`KismetSystemLibrary.GetObjectName` self) (`self.FacingPlayer?`) (`self.IsRunning`) false false 0.0 0.0 0 (`self.TargetLocation`) "+00000000.00:00:00.000000000" "NewEnumerator0" (struct :`Actor` "NewEnumerator0" :`MeshSettings` (struct) :`InspectionSettings` (struct :`InspectionPivotLocation` (0.0 0.0 0.0) :`Takeable` true :`InspectionAnimation` true :`InspectionAnimationSpeedSec` 0.5 :`InspectionBeginRotation` (struct) :`InspectionBeginScale` 1.0 :`MinZoomScale` 1.0 :`MaxZoomScale` 2.0 :`RotationSpeed` 2.5 :`SlideSpeed` 1.0 :`MaxSlideValue` 10.0 :`ItemName` "NSLOCTEXT(\"[B705432D9F56E45EAB380083611BB3A0]\", \"83C31BE444F430517147F699B94D0541\", \"Item Name\")" :`ItemInformation` "NSLOCTEXT(\"[B705432D9F56E45EAB380083611BB3A0]\", \"7F409F2D40820D83460EB48558FD30DA\", \"Item Information\")" :`ReadingText` "NSLOCTEXT(\"[B705432D9F56E45EAB380083611BB3A0]\", \"C15EC10546F1A784CEE5F683FE7F56D4\", \"Reading Text\")" :`TakeButton` (struct :`ButtonText` "NSLOCTEXT(\"[B705432D9F56E45EAB380083611BB3A0]\", \"3CBD47BD45DC3D763E4C2BBB0B6E509A\", \"Take\")") :`ExamineButton` (struct :`ButtonText` "NSLOCTEXT(\"[B705432D9F56E45EAB380083611BB3A0]\", \"8345B4934232439299CDD285AD198307\", \"Examine\")") :`ZoomPanButton` (struct :`ButtonText` "NSLOCTEXT(\"[B705432D9F56E45EAB380083611BB3A0]\", \"7857D3044307C1ACB0D8159A585378C7\", \"Zoom/Slide\")") :`DismissButton` (struct :`ButtonText` "NSLOCTEXT(\"[B705432D9F56E45EAB380083611BB3A0]\", \"0C5136C74698A97887F6BBB999475FB8\", \"Dismiss\")")) :`InventorySettings` (struct :`StorageType` "NewEnumerator3" :`NumberofItemstoAddInventory` 1 :`Interactable` true :`InteractionButton` (struct :`ButtonText` "NSLOCTEXT(\"[B705432D9F56E45EAB380083611BB3A0]\", \"68823F99438372835EA807A8E540726B\", \"Use\")") :`SwitchButton` (struct :`ButtonText` "NSLOCTEXT(\"[B705432D9F56E45EAB380083611BB3A0]\", \"CE4A86184BBD1D52D87B8DB04B10D919\", \"Switch\")") :`ZoomSlideButton` (struct :`ButtonText` "NSLOCTEXT(\"[B705432D9F56E45EAB380083611BB3A0]\", \"934F4D1B412728DCE3CC618995499657\", \"Zoom/Slide\")") :`CloseInventoryButton` (struct :`ButtonText` "NSLOCTEXT(\"[B705432D9F56E45EAB380083611BB3A0]\", \"CEF7F67643F304D28F2168921AFAEC24\", \"Close\")")) :`Pistol_MeshSettingsTop` (struct) :`Vhs_CurrentTime` "+00000000.00:00:00.000000000"))))

(event `/Game/LoryTest/Blueprints/Interface/MonsterInterface.ActionOnHearingSomething`
  (if (not (`self.IsRunning`))
    (`self.Toggle Walk/Run`)))

(event `/Game/HorrorEngine/Blueprints/Core/HorrorEngineInterface.RestoreSaveData`
  (params (AssetSave :type "/Game/HorrorEngine/Blueprints/Structures/SaveStructures/AssetsSave Structure"))
  (bind ((`BooleanSlot01_63_ED79FB5D49E9ED6768D7AE96EDFDE8DB` _booleanslot01) (`BooleanSlot02_64_3DE3E28A45CAE9F3E913659977556562` _booleanslot02) (`BooleanSlot03_65_04AA048C42686C9D2AF003962AEB7F6C` _booleanslot03) (`BooleanSlot04_66_3CB4510F40F5DDD3D81BCEA77398809A` _booleanslot04) (`FloatSlot01_62_3D225DB249A703592AAD5A8405C67C24` _floatslot01) (`FloatSlot02_72_0C6E79544AA699EC0216E1929F2FE1AC` _floatslot02) (`IntegerSlot01_75_ABA8053D4F033D11B1D4ECB38D77F6AB` _integerslot01) (`VectorSlot_88_ED6A62A541ECCAED428C6BA9C5D42119` _vectorslot)) (break `/Game/HorrorEngine/Blueprints/Structures/SaveStructures/AssetsSave` AssetSave))
  ;[0 1 0.5572] Save Settings
  (set `self.FacingPlayer?` _booleanslot01)
  (set `self.IsRunning` _booleanslot02)
  (set `self.TargetLocation` _vectorslot)
  (`self.TriggerGiveInvestigPos` (`self.TargetLocation`)))

(event `/Game/LoryTest/Blueprints/Interface/MonsterInterface.ActionOnReachingDestination`
  (if (`self.IsRunning`)
    (`self.Toggle Walk/Run`)))

(fn `UserConstructionScript`
  (`parent.UserConstructionScript`)
  (`PrimitiveComponent.SetCollisionEnabled` (`self.VisionConeMonster`) "NoCollision"))