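; An eight-digit security keypad that locks and unlocks connected cameras and alarms, with horror-event hooks.
; Pressed buttons animate and build a code shown through screen material textures; Enter checks it against the password.
; Player detection starts a warning timeline that raises the alarm unless the code is entered, also driving connected keycard controls.
; Repeated presses while unlocked can relock it, and lock, alarm and warning state is saved.
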(event `self.BeginLoad`
  ;[1 1 1] BeginPlay Settings
  (`|ExecutionSequence`
    (:`then_0`
      (for _array_element (`self.ConnectedCameras`)
        (set `/Game/HorrorEngine/Blueprints/UsableAssets/Electronics/SecurityCam.SecurityControlTarget` self _array_element)))
    (:`then_1`
      (for _array_element_2 (`self.ConnectedAlarms`)
        (set `/Game/HorrorEngine/Blueprints/UsableAssets/Electronics/SecurityAlarm.SecurityControlTarget` self _array_element_2)))))

(event `self.Use`
  (params (HorrorEvent :type Boolean))
  (bind _currentvalues (`self.CurrentValues`))
  ;[1 1 1] Use Panel Settings
  ;;[1 1 1] Select Button
  (`/Game/HorrorEngine/Blueprints/Core/HorrorEngineMacros.HM_CheckInteraction`)
  (bind _asmaster (`/Game/HorrorEngine/Blueprints/Core/HorrorEngineFunctions.GetPlayer`))
  (set `self.CurrentButton` (`/Game/HorrorEngine/HorrorEngine.HitComponent` _asmaster))
  ;;[1 1 1] Button Animation
  (`self.ButtonAnimation`)
  ;;[1 1 1] Locked or Not?
  (if (`self.Locked`)
    ;;[1 1 1] Pressed Reset/Enter or Digits?
    (if (or (== (`self.CurrentButton`) (`self.ButtonReset`)) (== (`self.CurrentButton`) (`self.ButtonEnter`)))
      ;;[1 1 1] Pressed Reset Button?
      (if (== (`self.CurrentButton`) (`self.ButtonReset`))
        ;;[1 1 1] Reset
        (set `self.CurrentValues` (`self.Reset`))
        (`self.DigitScreen`)
        (`self.Button Sound`)
        (set `self.EmptyButton` false)
        (else
          ;;[1 1 1] Entered 8 Digits?
          (if (== (`KismetArrayLibrary.Array_LastIndex` (`self.CurrentValues`)) 7)
            ;;[1 1 1] Correct Code?
            (if (== (+ (* (`|GetArrayItem` _currentvalues) 10000000) (* (`|GetArrayItem` _currentvalues 1) 1000000) (* (`|GetArrayItem` _currentvalues 2) 100000) (* (`|GetArrayItem` _currentvalues 3) 10000) (* (`|GetArrayItem` _currentvalues 4) 1000) (* (`|GetArrayItem` _currentvalues 5) 100) (* (`|GetArrayItem` _currentvalues 6) 10) (* (`|GetArrayItem` _currentvalues 7) 1)) (`self.8DigitPassword`))
              ;;[1 1 1] Unlock
              (`self.Unlock` false)
              (`self.Button Sound`)
              (`self.RemoveWarning`)
              (else
                ;;[1 1 1] Wrong Code
                (set `self.CurrentValues` (`self.Reset`) :!label _label)
                (`self.WrongScreen`)
                (set `self.EmptyButton` false)
                (`self.Button Sound`)
                (`self.Wrong Code Sound`)
                (`self.HorrorEventCheck` "NewEnumerator21")
                ;;[1 1 1] Alarm Counter
                (if (`self.AlarmAfterWrongCode`)
                  (set `self.AlarmCounter` (+ (`self.AlarmCounter`) 1))
                  (if (== 0 (`self.Alarm After (N) Times Wrong Code`))
                    (`self.Alarm` false)))))
            (else
              (goto _label)))))
      (else
        ;;[1 1 1] Already Entered 8 Digits?
        (if (>= (`KismetArrayLibrary.Array_LastIndex` (`self.CurrentValues`)) 7)
          ;;[1 1 1] Disable Digital Button Sound
          (set `self.EmptyButton` true)
          (`self.Button Sound`)
          (else
            ;;[1 1 1] Calculate Digits
            (`KismetArrayLibrary.Array_Add` (`self.CurrentValues`) (`KismetStringLibrary.Conv_StringToInt` (`KismetStringLibrary.Conv_NameToString` (`|GetArrayItem` (`ActorComponent.ComponentTags` (`self.CurrentButton`))))))
            (`self.DigitScreen`)
            (set `self.EmptyButton` false)
            (`self.Button Sound`)))))
    (else
      ;;[1 1 1] Check for Lock Again
      (`self.Button Sound`)
      (`|ExecutionSequence`
        (:`then_0`
          (`KismetSystemLibrary.RetriggerableDelay` 3.0)
          (set `self.ResetButtonCounter` 0))
        (:`then_1`
          (if (== (`self.CurrentButton`) null)
            (bind _output_get (set `self.ResetButtonCounter` (+ (`self.ResetButtonCounter`) 1)))
            (if (== _output_get (`self.Press Reset (N) Times to Lock`))
              (`self.Lock` false))))))))

(event `WrongScreen`
  ;[1 1 1] Digit Screen Settings
  (`|ExecutionSequence`
    (:`then_0`
      (`KismetSystemLibrary.Delay` 0.2)
      (set `self.InteractionEnabled` false)
      (`KismetSystemLibrary.Delay` 0.8)
      (set `self.InteractionEnabled` true)
      (set `self.CurrentScreen` null))
    (:`then_1`
      (set `self.CurrentScreenGlow` 100.0)
      (set `self.CurrentScreen` "/Game/HorrorEngine/Textures/Digit_Wrong.Digit_Wrong")))
  (bind _returnvalue (`PrimitiveComponent.CreateDynamicMaterialInstance` (`self.SecurityControl`) 1 "/Game/HorrorEngine/Materials/HE_ControlScreen.HE_ControlScreen" "None" :!label _label_2))
  (`MaterialInstanceDynamic.SetTextureParameterValue` _returnvalue "Texture" (`self.CurrentScreen`))
  (`MaterialInstanceDynamic.SetScalarParameterValue` _returnvalue "Emissive" (`self.CurrentScreenGlow`)))

(event `CorrectScreen`
  ;[1 1 1] Digit Screen Settings
  (set `self.CurrentScreenGlow` 20.0)
  (set `self.CurrentScreen` "/Game/HorrorEngine/Textures/Digit_Open.Digit_Open")
  (goto _label_2))

(event `DigitScreen`
  ;[1 1 1] Digit Screen Settings
  (set `self.CurrentScreenGlow` 100.0)
  (set `self.CurrentScreen` (select `int` (+ (`KismetArrayLibrary.Array_LastIndex` (`self.CurrentValues`)) 1) :`0` "/Game/LoryTest/Textures/8Digit_0.8Digit_0" :`1` "/Game/LoryTest/Textures/8Digit_1.8Digit_1" :`2` "/Game/LoryTest/Textures/8Digit_2.8Digit_2" :`3` "/Game/LoryTest/Textures/8Digit_3.8Digit_3" :`4` "/Game/LoryTest/Textures/8Digit_4.8Digit_4" :`5` "/Game/LoryTest/Textures/8Digit_5.8Digit_5" :`6` "/Game/LoryTest/Textures/8Digit_6.8Digit_6" :`7` "/Game/LoryTest/Textures/8Digit_7.8Digit_7" :`8` "/Game/LoryTest/Textures/8Digit_8.8Digit_8" :!type "Texture Object Reference"))
  (goto _label_2))

(event `ButtonAnimation`
  (bind _currentbutton (`self.CurrentButton`))
  (bind (_relativelocation_x _relativelocation_y _relativelocation_z) (`KismetMathLibrary.BreakVector` (`SceneComponent.RelativeLocation` _currentbutton)))
  ;[1 1 1] Button Animation Settings
  (set `self.InteractionEnabled` false)
  (bind (_direction _animation) (`Timeline|ButtonTimeline_0` :!via `PlayFromStart`)
    (:`Update`
      (if (`KismetSystemLibrary.IsValid` _currentbutton)
        (`SceneComponent.K2_SetRelativeLocation` _currentbutton (`KismetMathLibrary.MakeVector` _relativelocation_x (`KismetMathLibrary.Lerp` 2.0 1.6 _animation) _relativelocation_z) false false)))
    (:`Finished`
      (set `self.InteractionEnabled` true))))

(event `Button Sound`
  (bind _returnvalue (select `bool` (`self.EmptyButton`) :`false` (`self.ButtonSound`) :`true` (`self.EmptyButtonSound`)))
  ;[1 1 1] Sound Settings
  (`/Game/HorrorEngine/Blueprints/Core/HorrorEngineMacros.HM_3DSound` _returnvalue false _returnvalue null (`self.SoundAttenuation`)))

(event `self.Lock`
  (params (HorrorEvent :type Boolean))
  ;[1 1 1] Lock / Unlock Settings
  (set `self.CurrentValues` (`self.Reset`))
  (`self.DigitScreen`)
  (`self.Wrong Code Sound`)
  (set `self.Locked` true)
  (set `self.EmptyButton` false)
  (`self.Open/On` (`self.ConnectedCameras`) false)
  (`self.Open/On` (`self.ConnectedAlarms`) false)
  (`self.HorrorEventCheck` "NewEnumerator5"))

(event `Wrong Code Sound`
  (bind _wrongcodesound (`self.WrongCodeSound`))
  ;[1 1 1] Sound Settings
  (`/Game/HorrorEngine/Blueprints/Core/HorrorEngineMacros.HM_3DSound` _wrongcodesound false _wrongcodesound null (`self.SoundAttenuation`)))

(event `self.Unlock`
  (params (HorrorEvent :type Boolean))
  ;[1 1 1] Lock / Unlock Settings
  (`/Game/HorrorEngine/Blueprints/Core/HorrorEngineMacros.HM_Stop3DSound` (`self.WarningSound`))
  (`self.CorrectScreen`)
  (`self.Correct Code Sound`)
  (set `self.Locked` false)
  (set `self.EmptyButton` true)
  (`self.Close/Off` (`self.ConnectedCameras`) false)
  (`self.Close/Off` (`self.ConnectedAlarms`) false)
  (set `self.AlarmCounter` 0)
  (`self.Disalarm` false)
  (`self.HorrorEventCheck` "NewEnumerator6"))

(event `Correct Code Sound`
  (bind _correctcodesound (`self.CorrectCodeSound`))
  ;[1 1 1] Sound Settings
  (`/Game/HorrorEngine/Blueprints/Core/HorrorEngineMacros.HM_3DSound` _correctcodesound false _correctcodesound null (`self.SoundAttenuation`)))

(event `self.Alarm`
  (params (HorrorEvent :type Boolean))
  (bind _connectedkeycardcontrols (`self.ConnectedKeycardControls`))
  ;[1 1 1] Alarm Settings
  (if (not (`self.AlarmStarted`))
    (set `self.AlarmStarted` true)
    (if (not (`self.Locked`))
      (`self.Lock` false))
    (`self.AlarmSound`)
    (`self.Alarm` (`self.ConnectedAlarms`) false)
    (`self.HorrorEventCheck` "NewEnumerator23")
    (`self.Close/Off` _connectedkeycardcontrols false)
    (for _array_element _connectedkeycardcontrols
      (set `/Game/HorrorEngine/Blueprints/UsableAssets/Electronics/KeycardControl.Disalarmed` false _array_element))))

(event `Warning Sound`
  (bind _warningsound (`self.WarningSound`))
  ;[1 1 1] Sound Settings
  (`/Game/HorrorEngine/Blueprints/Core/HorrorEngineMacros.HM_3DSound` _warningsound false _warningsound null (`self.SoundAttenuation`)))

(event `self.Disalarm`
  (params (HorrorEvent :type Boolean))
  ;[1 1 1] Alarm Settings
  (if (`self.AlarmStarted`)
    (set `self.AlarmStarted` true)
    (`/Game/HorrorEngine/Blueprints/Core/HorrorEngineMacros.HM_Stop3DSound` (`self.Alarm Sound`))
    (`self.Disalarm` (`self.ConnectedAlarms`) false)
    (`self.HorrorEventCheck` "NewEnumerator24")
    (for _array_element (`self.ConnectedKeycardControls`)
      (set `/Game/HorrorEngine/Blueprints/UsableAssets/Electronics/KeycardControl.Disalarmed` true _array_element))))

(event `AlarmSound`
  (bind _alarm_sound (`self.Alarm Sound`))
  ;[1 1 1] Sound Settings
  (`/Game/HorrorEngine/Blueprints/Core/HorrorEngineMacros.HM_3DSound` _alarm_sound false _alarm_sound null (`self.SoundAttenuation`)))

(event `PlayerDetected`
  ;[1 1 1] Detection Settings
  (if (`self.Locked`)
    (if (not (`self.AlarmStarted`))
      (`self.HorrorEventCheck` "NewEnumerator22")
      (`self.Warning Sound` :!label _label_3)
      (set `self.Detected` true)
      (bind (_direction _remainingtime) (`Timeline|WarningTimeline_0` :`NewTime` (`self.WarningTime`) :!label _label_4)
        (:`Update`
          (set `self.WarningTime` _remainingtime))
        (:`Alarm`
          (`/Game/HorrorEngine/Blueprints/Core/HorrorEngineMacros.HM_Stop3DSound` (`self.WarningSound`))
          (`self.Alarm` false)
          (`self.RemoveWarning`))))))

(event `Warning`
  ;[1 1 1] Detection Settings
  (goto _label_3))

(event `RemoveWarning`
  ;[1 1 1] Detection Settings
  (set `self.Detected` false)
  (set `self.WarningTime` 0.0)
  (`|ExecutionSequence`
    (:`then_0`
      (goto _label_4 :!via `Stop`))
    (:`then_1`
      (goto _label_4 :!via `SetNewTime`))))

(event `self.CollectSaveData`
  ;[0 1 0.5572] Save Settings
  (bind _asmaster (`/Game/HorrorEngine/Blueprints/Core/HorrorEngineFunctions.GetPlayer`))
  (`KismetArrayLibrary.Array_Add` (`/Game/HorrorEngine/Blueprints/Core/HE_SaveGameComponent.AssetCache` (`/Game/HorrorEngine/HorrorEngine.HE_SaveGameComponent` _asmaster)) (make `/Game/HorrorEngine/Blueprints/Structures/SaveStructures/AssetsSave` (`KismetSystemLibrary.GetObjectName` self) (`self.Locked`) (`self.EmptyButton`) (`self.AlarmStarted`) (`self.Detected`) (`self.WarningTime`) 0.0 (`self.AlarmCounter`) "+00000000.00:00:00.000000000" "NewEnumerator0" (struct :`Actor` "NewEnumerator0" :`MeshSettings` (struct) :`InspectionSettings` (struct :`InspectionPivotLocation` (0.0 0.0 0.0) :`Takeable` true :`InspectionAnimation` true :`InspectionAnimationSpeedSec` 0.5 :`InspectionBeginRotation` (struct) :`InspectionBeginScale` 1.0 :`MinZoomScale` 1.0 :`MaxZoomScale` 2.0 :`RotationSpeed` 2.5 :`SlideSpeed` 1.0 :`MaxSlideValue` 10.0 :`ItemName` "NSLOCTEXT(\"[72D96A71A5A8AE557F2CF85BCADED4C7]\", \"E57FFDD74966D5F82BF63883ABA82555\", \"Item Name\")" :`ItemInformation` "NSLOCTEXT(\"[72D96A71A5A8AE557F2CF85BCADED4C7]\", \"EB70A4A44FD5676F4CF65FB8DA871D72\", \"Item Information\")" :`ReadingText` "NSLOCTEXT(\"[72D96A71A5A8AE557F2CF85BCADED4C7]\", \"E8DF7D57474712F6B44220833329CB33\", \"Reading Text\")" :`TakeButton` (struct :`ButtonText` "NSLOCTEXT(\"[72D96A71A5A8AE557F2CF85BCADED4C7]\", \"8D39A70F469D561F105C998340432531\", \"Take\")") :`ExamineButton` (struct :`ButtonText` "NSLOCTEXT(\"[72D96A71A5A8AE557F2CF85BCADED4C7]\", \"378B741B447B08B951599486A659A8B3\", \"Examine\")") :`ZoomPanButton` (struct :`ButtonText` "NSLOCTEXT(\"[72D96A71A5A8AE557F2CF85BCADED4C7]\", \"A8767EAD4C9AEAC79B443792884F319B\", \"Zoom/Slide\")") :`DismissButton` (struct :`ButtonText` "NSLOCTEXT(\"[72D96A71A5A8AE557F2CF85BCADED4C7]\", \"EF448097457973344CCDDCB8C3E28A11\", \"Dismiss\")")) :`InventorySettings` (struct :`StorageType` "NewEnumerator3" :`NumberofItemstoAddInventory` 1 :`Interactable` true :`InteractionButton` (struct :`ButtonText` "NSLOCTEXT(\"[72D96A71A5A8AE557F2CF85BCADED4C7]\", \"DC4C7F854D49832FE1572D95EC871DC2\", \"Use\")") :`SwitchButton` (struct :`ButtonText` "NSLOCTEXT(\"[72D96A71A5A8AE557F2CF85BCADED4C7]\", \"B2CD80E24EACFBA7714229A886F0FE62\", \"Switch\")") :`ZoomSlideButton` (struct :`ButtonText` "NSLOCTEXT(\"[72D96A71A5A8AE557F2CF85BCADED4C7]\", \"6BBBF38145EE84CDFFFAEDA553566755\", \"Zoom/Slide\")") :`CloseInventoryButton` (struct :`ButtonText` "NSLOCTEXT(\"[72D96A71A5A8AE557F2CF85BCADED4C7]\", \"E82B31274C73EC54753714BA51178EA9\", \"Close\")")) :`Pistol_MeshSettingsTop` (struct) :`Vhs_CurrentTime` "+00000000.00:00:00.000000000"))))

(event `self.RestoreSaveData`
  (params (AssetSave :type "/Game/HorrorEngine/Blueprints/Structures/SaveStructures/AssetsSave Structure"))
  (bind ((`BooleanSlot01_63_ED79FB5D49E9ED6768D7AE96EDFDE8DB` _booleanslot01) (`BooleanSlot02_64_3DE3E28A45CAE9F3E913659977556562` _booleanslot02) (`BooleanSlot03_65_04AA048C42686C9D2AF003962AEB7F6C` _booleanslot03) (`BooleanSlot04_66_3CB4510F40F5DDD3D81BCEA77398809A` _booleanslot04) (`FloatSlot01_62_3D225DB249A703592AAD5A8405C67C24` _floatslot01) (`FloatSlot02_72_0C6E79544AA699EC0216E1929F2FE1AC` _floatslot02) (`IntegerSlot01_75_ABA8053D4F033D11B1D4ECB38D77F6AB` _integerslot01)) (break `/Game/HorrorEngine/Blueprints/Structures/SaveStructures/AssetsSave` AssetSave))
  ;[0 1 0.5572] Save Settings
  (set `self.Locked` _booleanslot01)
  (set `self.EmptyButton` _booleanslot02)
  (set `self.AlarmStarted` _booleanslot03)
  (set `self.Detected` _booleanslot04)
  (set `self.WarningTime` _floatslot01)
  (set `self.AlarmCounter` _integerslot01)
  (`self.BeginLoad`)
  (if (`self.Detected`)
    (`TimelineComponent.SetNewTime` (`self.WarningTimeline_0`) (`self.WarningTime`))
    (`self.Warning`)
    (elif (`self.AlarmStarted`)
      (`self.AlarmSound`)
      (elif (not (`self.Locked`))
        (`self.CorrectScreen`)))))

(fn `UserConstructionScript`
  (`/Game/HorrorEngine/Blueprints/Core/HorrorEngineMacros.HM_DefaultConstructions` (`self.CreateNewHorrorEvent`))
  (`/Game/HorrorEngine/Blueprints/Core/HorrorEngineFunctions.PlayRate` (`self.WarningTimeline_0`) (`self.DetectionWarningDuration(Sec)`))
  (bind _returnvalue (`PrimitiveComponent.CreateDynamicMaterialInstance` (`self.Button1`) 0 "/Game/HorrorEngine/Materials/HE_LockPanelButton.HE_LockPanelButton" "None"))
  (`MaterialInstanceDynamic.SetTextureParameterValue` _returnvalue "Button" "/Game/HorrorEngine/Textures/Button_1.Button_1")
  (bind _returnvalue_2 (`PrimitiveComponent.CreateDynamicMaterialInstance` (`self.Button2`) 0 "/Game/HorrorEngine/Materials/HE_LockPanelButton.HE_LockPanelButton" "None"))
  (`MaterialInstanceDynamic.SetTextureParameterValue` _returnvalue_2 "Button" "/Game/HorrorEngine/Textures/Button_2.Button_2")
  (bind _returnvalue_3 (`PrimitiveComponent.CreateDynamicMaterialInstance` (`self.Button3`) 0 "/Game/HorrorEngine/Materials/HE_LockPanelButton.HE_LockPanelButton" "None"))
  (`MaterialInstanceDynamic.SetTextureParameterValue` _returnvalue_3 "Button" "/Game/HorrorEngine/Textures/Button_3.Button_3")
  (bind _returnvalue_4 (`PrimitiveComponent.CreateDynamicMaterialInstance` (`self.Button4`) 0 "/Game/HorrorEngine/Materials/HE_LockPanelButton.HE_LockPanelButton" "None"))
  (`MaterialInstanceDynamic.SetTextureParameterValue` _returnvalue_4 "Button" "/Game/HorrorEngine/Textures/Button_4.Button_4")
  (bind _returnvalue_5 (`PrimitiveComponent.CreateDynamicMaterialInstance` (`self.Button5`) 0 "/Game/HorrorEngine/Materials/HE_LockPanelButton.HE_LockPanelButton" "None"))
  (`MaterialInstanceDynamic.SetTextureParameterValue` _returnvalue_5 "Button" "/Game/HorrorEngine/Textures/Button_5.Button_5")
  (bind _returnvalue_6 (`PrimitiveComponent.CreateDynamicMaterialInstance` (`self.Button6`) 0 "/Game/HorrorEngine/Materials/HE_LockPanelButton.HE_LockPanelButton" "None"))
  (`MaterialInstanceDynamic.SetTextureParameterValue` _returnvalue_6 "Button" "/Game/HorrorEngine/Textures/Button_6.Button_6")
  (bind _returnvalue_7 (`PrimitiveComponent.CreateDynamicMaterialInstance` (`self.Button7`) 0 "/Game/HorrorEngine/Materials/HE_LockPanelButton.HE_LockPanelButton" "None"))
  (`MaterialInstanceDynamic.SetTextureParameterValue` _returnvalue_7 "Button" "/Game/HorrorEngine/Textures/Button_7.Button_7")
  (bind _returnvalue_8 (`PrimitiveComponent.CreateDynamicMaterialInstance` (`self.Button8`) 0 "/Game/HorrorEngine/Materials/HE_LockPanelButton.HE_LockPanelButton" "None"))
  (`MaterialInstanceDynamic.SetTextureParameterValue` _returnvalue_8 "Button" "/Game/HorrorEngine/Textures/Button_8.Button_8")
  (bind _returnvalue_9 (`PrimitiveComponent.CreateDynamicMaterialInstance` (`self.Button9`) 0 "/Game/HorrorEngine/Materials/HE_LockPanelButton.HE_LockPanelButton" "None"))
  (`MaterialInstanceDynamic.SetTextureParameterValue` _returnvalue_9 "Button" "/Game/HorrorEngine/Textures/Button_9.Button_9")
  (bind _returnvalue_10 (`PrimitiveComponent.CreateDynamicMaterialInstance` (`self.ButtonReset`) 0 "/Game/HorrorEngine/Materials/HE_LockPanelButton.HE_LockPanelButton" "None"))
  (`MaterialInstanceDynamic.SetTextureParameterValue` _returnvalue_10 "Button" "/Game/HorrorEngine/Textures/Button_Reset.Button_Reset")
  (bind _returnvalue_11 (`PrimitiveComponent.CreateDynamicMaterialInstance` (`self.Button0`) 0 "/Game/HorrorEngine/Materials/HE_LockPanelButton.HE_LockPanelButton" "None"))
  (`MaterialInstanceDynamic.SetTextureParameterValue` _returnvalue_11 "Button" "/Game/HorrorEngine/Textures/Button_0.Button_0")
  (bind _returnvalue_12 (`PrimitiveComponent.CreateDynamicMaterialInstance` (`self.ButtonEnter`) 0 "/Game/HorrorEngine/Materials/HE_LockPanelButton.HE_LockPanelButton" "None"))
  (`MaterialInstanceDynamic.SetTextureParameterValue` _returnvalue_12 "Button" "/Game/HorrorEngine/Textures/Button_Enter.Button_Enter"))