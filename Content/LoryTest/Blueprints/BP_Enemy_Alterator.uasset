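; Alterator enemy that applies a random slow, dizzy or zoom effect to the player on entering its vision cone.
; Effects are child-actor GameplaySettingsModifiers switched on and off, with attack and cooldown timings read from DT_Alternator_Effects.
; An attack, cooldown and range-check loop repeats attacks while the player stays in range.
; It registers its state with the player's save component and resumes attack or cooldown on restore.
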(event `/Game/HorrorEngine/Blueprints/Core/HorrorEngineInterface.CollectSaveData`
  ;[0 1 0.5572] Save Settings
  (bind _asmaster (`/Game/HorrorEngine/Blueprints/Core/HorrorEngineFunctions.GetPlayer`))
  (`KismetArrayLibrary.Array_Add` (`/Game/HorrorEngine/Blueprints/Core/HE_SaveGameComponent.AssetCache` (`/Game/HorrorEngine/HorrorEngine.HE_SaveGameComponent` _asmaster)) (make `/Game/HorrorEngine/Blueprints/Structures/SaveStructures/AssetsSave` (`KismetSystemLibrary.GetObjectName` self) (`self.FacingPlayer?`) (`self.IsRunning`) (`self.Attacking`) (`self.Cooldown`) (`self.PlayerinRange`) 0.0 0.0 0 (`self.TargetLocation`) "+00000000.00:00:00.000000000" "NewEnumerator0" (struct :`Actor` "NewEnumerator0" :`MeshSettings` (struct) :`InspectionSettings` (struct :`InspectionPivotLocation` (0.0 0.0 0.0) :`Takeable` true :`InspectionAnimation` true :`InspectionAnimationSpeedSec` 0.5 :`InspectionBeginRotation` (struct) :`InspectionBeginScale` 1.0 :`MinZoomScale` 1.0 :`MaxZoomScale` 2.0 :`RotationSpeed` 2.5 :`SlideSpeed` 1.0 :`MaxSlideValue` 10.0 :`ItemName` "NSLOCTEXT(\"[61071E7DE69A920A18AAD1F49B67E737]\", \"BB9A20AF4AA4CE3A2754E69E4BE0E58A\", \"Item Name\")" :`ItemInformation` "NSLOCTEXT(\"[61071E7DE69A920A18AAD1F49B67E737]\", \"D1324C91439B7B7859E7A7B23251D35E\", \"Item Information\")" :`ReadingText` "NSLOCTEXT(\"[61071E7DE69A920A18AAD1F49B67E737]\", \"7043C4A5478C4165C1890986A92E06E3\", \"Reading Text\")" :`TakeButton` (struct :`ButtonText` "NSLOCTEXT(\"[61071E7DE69A920A18AAD1F49B67E737]\", \"E9BC3E094CC2B8E12C0158A0630163D7\", \"Take\")") :`ExamineButton` (struct :`ButtonText` "NSLOCTEXT(\"[61071E7DE69A920A18AAD1F49B67E737]\", \"9ED23ED64147F1153C965B9781239CA5\", \"Examine\")") :`ZoomPanButton` (struct :`ButtonText` "NSLOCTEXT(\"[61071E7DE69A920A18AAD1F49B67E737]\", \"4A47D62D4BA3F014FB088081DC03E149\", \"Zoom/Slide\")") :`DismissButton` (struct :`ButtonText` "NSLOCTEXT(\"[61071E7DE69A920A18AAD1F49B67E737]\", \"89405D834488472C8AE4089722740AD0\", \"Dismiss\")")) :`InventorySettings` (struct :`StorageType` "NewEnumerator3" :`NumberofItemstoAddInventory` 1 :`Interactable` true :`InteractionButton` (struct :`ButtonText` "NSLOCTEXT(\"[61071E7DE69A920A18AAD1F49B67E737]\", \"F04EA2554FEA9883300C62A5D6DB02F7\", \"Use\")") :`SwitchButton` (struct :`ButtonText` "NSLOCTEXT(\"[61071E7DE69A920A18AAD1F49B67E737]\", \"EA8176DD40ADE422FE225D93BD42A10F\", \"Switch\")") :`ZoomSlideButton` (struct :`ButtonText` "NSLOCTEXT(\"[61071E7DE69A920A18AAD1F49B67E737]\", \"0BE155D544CF288B09DA57A81A1CE8B5\", \"Zoom/Slide\")") :`CloseInventoryButton` (struct :`ButtonText` "NSLOCTEXT(\"[61071E7DE69A920A18AAD1F49B67E737]\", \"3EF1E4EE46DA0A71FF6F27A4DB1BC5AA\", \"Close\")")) :`Pistol_MeshSettingsTop` (struct) :`Vhs_CurrentTime` "+00000000.00:00:00.000000000") (`self.AttackEffect`))))

(event `SlowEffect`
  ;[1 1 1] Effects
  (bind _output_get (set `self.ActiveComponent` (`self.Slow Effect`)))
  (`self.ActivateEffect` _output_get))

(event `SpinThatHeadCrazy`
  ;[1 1 1] Effects
  (bind _output_get (set `self.ActiveComponent` (`self.Headache`)))
  (`self.ActivateEffect` _output_get))

(event `/Game/HorrorEngine/Blueprints/Core/HorrorEngineInterface.RestoreSaveData`
  (params (AssetSave :type "/Game/HorrorEngine/Blueprints/Structures/SaveStructures/AssetsSave Structure"))
  (bind ((`BooleanSlot01_63_ED79FB5D49E9ED6768D7AE96EDFDE8DB` _booleanslot01) (`BooleanSlot02_64_3DE3E28A45CAE9F3E913659977556562` _booleanslot02) (`BooleanSlot03_65_04AA048C42686C9D2AF003962AEB7F6C` _booleanslot03) (`BooleanSlot04_66_3CB4510F40F5DDD3D81BCEA77398809A` _booleanslot04) (`BooleanSlot05_95_36200D344B0D0C7AFF1521A5B1426E07` _booleanslot05) (`FloatSlot01_62_3D225DB249A703592AAD5A8405C67C24` _floatslot01) (`FloatSlot02_72_0C6E79544AA699EC0216E1929F2FE1AC` _floatslot02) (`IntegerSlot01_75_ABA8053D4F033D11B1D4ECB38D77F6AB` _integerslot01) (`VectorSlot_88_ED6A62A541ECCAED428C6BA9C5D42119` _vectorslot) (`TimespanSlot01_78_45954CE745E761DBE5FA658D05AFB6AE` _timespanslot01) (`OldTvSource_81_D05C908C4A423C80CC5CC1B8EC706C06` _oldtvsource) (`InsertedVhs_85_53C61BCD458712DC2E01A8B46D51201F` _insertedvhs) (`AlternatorEffect_92_1753BD2D4341797E6AD99094E6E56FE6` _alternatoreffect)) (break `/Game/HorrorEngine/Blueprints/Structures/SaveStructures/AssetsSave` AssetSave))
  (bind _activecomponent (`self.ActiveComponent`))
  ;[0 1 0.5572] Save Settings
  (set `self.FacingPlayer?` _booleanslot01)
  (set `self.IsRunning` _booleanslot02)
  (set `self.Attacking` _booleanslot03)
  (set `self.Cooldown` _booleanslot04)
  (set `self.PlayerinRange` _booleanslot05)
  (set `self.TargetLocation` _vectorslot)
  (set `self.AttackEffect` _alternatoreffect)
  (`self.TriggerGiveInvestigPos` (`self.TargetLocation`))
  (if (`self.Attacking`)
    ;[1 1 1] Effect Trigger
    (bind (_attackduration _cooldownduration) (`self.SetAndShoot` :!label _label))
    (`KismetSystemLibrary.Delay` _attackduration)
    (`/Engine/EditorBlueprintResources/StandardMacros.IsValid` _activecomponent
      (:`Is Valid`
        (`self.DeactivateEffect` _activecomponent))
      (:`Is Not Valid`
        _))
    (set `self.Attacking` false)
    (set `self.Cooldown` true)
    (`KismetSystemLibrary.Delay` _cooldownduration)
    (set `self.Cooldown` false)
    (if (`self.PlayerinRange`)
      (if (and (== (stale `self.VisionConeMonster.OnComponentBeginOverlap` OtherActor) (`GameplayStatics.GetPlayerCharacter` 0)) (not (`self.Cooldown`)) (not (`self.Attacking`))) :!label _label_2
        (set `self.PlayerinRange` true :!label _label_3)
        (set `self.Attacking` true)
        (goto _label)))
    (else
      (if (`self.Cooldown`)
        (bind _cooldownvalue (`self.Get CooldownTimer` (`self.AttackEffect`)))
        (`KismetSystemLibrary.Delay` _cooldownvalue)
        (set `self.Cooldown` false))
      (if (`self.FacingPlayer?`)
        (goto _label_3)))))

(event `Can't See Shit`
  ;[1 1 1] Effects
  (bind _output_get (set `self.ActiveComponent` (`self.Zoom`)))
  (`self.ActivateEffect` _output_get))

(event `self.VisionConeMonster.OnComponentBeginOverlap`
  (params (OverlappedComponent :type "PrimitiveComponent Object Reference") (OtherActor :type "Actor Object Reference") (OtherComp :type "PrimitiveComponent Object Reference") (OtherBodyIndex :type Integer) (bFromSweep :type Boolean) (SweepResult :type "HitResult Structure (by ref)"))
  ;[1 1 1] Effect Trigger
  (goto _label_2))

(event `self.VisionConeMonster.OnComponentEndOverlap`
  (params (OverlappedComponent :type "PrimitiveComponent Object Reference") (OtherActor :type "Actor Object Reference") (OtherComp :type "PrimitiveComponent Object Reference") (OtherBodyIndex :type Integer))
  (set `self.PlayerinRange` false))

(fn `ActivateEffect`
  (params (EffectComponent :type "ChildActorComponent Object Reference"))
  (bind _asgameplay_settings_modifier (cast `/Game/HorrorEngine/Blueprints/UsableAssets/PortalAndTriggers/GameplaySettingsModifier` (`ChildActorComponent.ChildActor` EffectComponent)))
  (`/Game/HorrorEngine/Blueprints/Core/Use.Open/On` _asgameplay_settings_modifier false)
  (`KismetSystemLibrary.PrintString` (`KismetStringLibrary.Concat_StrStr` (`KismetSystemLibrary.GetObjectName` EffectComponent) " Activated")))

(fn `DeactivateEffect`
  (params (`Effect Component` :type "ChildActorComponent Object Reference"))
  (bind _childactor (`ChildActorComponent.ChildActor` `Effect Component`))
  (bind _asgameplay_settings_modifier (cast `/Game/HorrorEngine/Blueprints/UsableAssets/PortalAndTriggers/GameplaySettingsModifier` _childactor)
    (:`then`
      (`/Game/HorrorEngine/Blueprints/Core/Use.Close/Off` _asgameplay_settings_modifier false)
      (`KismetSystemLibrary.PrintString` (`KismetStringLibrary.Concat_StrStr` (`KismetSystemLibrary.GetObjectName` _childactor) " Deactivated"))
      (set `self.ActiveComponent` null))
    (:`CastFailed`
      (`KismetSystemLibrary.PrintString` "Nothing to Deactivate"))))

(fn `Get CooldownTimer`
  (params (ActiveEffect :type "/Game/LoryTest/Blueprints/Alternator_effects Enum" :default "NewEnumerator0"))
  (returns (CoolDownValue :type "Float (double-precision)"))
  (bind _outrownames (`DataTableFunctionLibrary.GetDataTableRowNames` "/Game/LoryTest/Blueprints/DT_Alternator_Effects.DT_Alternator_Effects"))
  (bind _returnvalue (`|GetDataTableRow` "/Game/LoryTest/Blueprints/DT_Alternator_Effects.DT_Alternator_Effects" (`|GetArrayItem` _outrownames (`KismetMathLibrary.Conv_ByteToInt` ActiveEffect)))
    (:`then`
      _)
    (:`RowNotFound`
      (`KismetSystemLibrary.PrintString` "Couldn't locate row value")))
  (return (`.Cooldown_15_E075F4384261FBFDB548E5A2B0E6A165` (break `/Game/LoryTest/Blueprints/Alternator_Effects_Values` _returnvalue))))

(fn `SetAndShoot`
  (returns (AttackDuration :type "Float (double-precision)") (CooldownDuration :type "Float (double-precision)"))
  (bind _returnvalue (`KismetMathLibrary.RandomIntegerInRange` 0 2))
  (set `self.EffectIndexInUse` _returnvalue)
  (bind _output_get (set `self.AttackEffect` (select `int` _returnvalue :`0` "NewEnumerator0" :`1` "NewEnumerator1" :`2` "NewEnumerator2" :!type "/Game/LoryTest/Blueprints/Alternator_effects Enum")))
  (bind _outrownames (`DataTableFunctionLibrary.GetDataTableRowNames` "/Game/LoryTest/Blueprints/DT_Alternator_Effects.DT_Alternator_Effects"))
  (bind _returnvalue_2 (`|GetDataTableRow` "/Game/LoryTest/Blueprints/DT_Alternator_Effects.DT_Alternator_Effects" (`|GetArrayItem` _outrownames _returnvalue))
    (:`then`
      (switch `/Game/LoryTest/Blueprints/Alternator_effects` _output_get
        (:`NewEnumerator0`
          (`self.SlowEffect`))
        (:`NewEnumerator1`
          (`self.SpinThatHeadCrazy`))
        (:`NewEnumerator2`
          (`self.Can't See Shit`)))
      (bind (_name _duration _cooldown) (break `/Game/LoryTest/Blueprints/Alternator_Effects_Values` _returnvalue_2))
      (return _duration _cooldown))))

(fn `UserConstructionScript`
  (`parent.UserConstructionScript`))