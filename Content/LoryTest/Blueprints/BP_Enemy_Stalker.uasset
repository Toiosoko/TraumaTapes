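; BP_Enemy_Stalker is an enemy that halts while the player looks at it, unless the player is close enough to trigger a chase.
; ToggleMovement records the look state and stops or starts movement, ignoring stop requests while ChasePlayer is set.
; The CheckPlayerDistance overlap sets ChasePlayer and starts movement when the player enters.
; Leaving clears the flag without stopping movement directly.
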(event `/Game/LoryTest/Blueprints/Interface/MovementInterface.ToggleMovement`
  (params (ReasonToStop :type Boolean))
  (if (`self.ChasePlayer`)
    (`self.StartMovement` :!label _label)
    (elif ReasonToStop
      (set `self.PlayerLookingAtMe` true)
      (`self.StopMovement`)
      (else
        (set `self.PlayerLookingAtMe` false)
        (goto _label)))))

(event `self.CheckPlayerDistance.OnComponentBeginOverlap`
  (params (OverlappedComponent :type "PrimitiveComponent Object Reference") (OtherActor :type "Actor Object Reference") (OtherComp :type "PrimitiveComponent Object Reference") (OtherBodyIndex :type Integer) (bFromSweep :type Boolean) (SweepResult :type "HitResult Structure (by ref)"))
  (if (== OtherActor (`GameplayStatics.GetPlayerCharacter` 0))
    (set `self.ChasePlayer` true)
    (`self.StartMovement`)))

(event `self.CheckPlayerDistance.OnComponentEndOverlap`
  (params (OverlappedComponent :type "PrimitiveComponent Object Reference") (OtherActor :type "Actor Object Reference") (OtherComp :type "PrimitiveComponent Object Reference") (OtherBodyIndex :type Integer))
  (if (== OtherActor (`GameplayStatics.GetPlayerCharacter` 0))
    (set `self.ChasePlayer` false)))

(fn `UserConstructionScript`
  (`parent.UserConstructionScript`))