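; BP_EnemyAi is an enemy pawn that chases the player once it sees them.
; Its PawnSensing component's OnSeePawn event checks for player pawn 0, sets IsSeeingPlayer and calls FollowPlayer.
; FollowPlayer issues an AI Move To toward the player with stop-on-overlap enabled.
; The flag is never cleared after a sighting, as the only reset runs when it is already false.
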(event `self.PawnSensing.OnSeePawn`
  (params (Pawn :type "Pawn Object Reference"))
  (if (== Pawn (`GameplayStatics.GetPlayerPawn` 0))
    (set `self.IsSeeingPlayer?` true)
    (`self.FollowPlayer`)))

(event `FollowPlayer`
  (if (`self.IsSeeingPlayer?`)
    (`|AIMoveTo` self (0.0 0.0 0.0) (`GameplayStatics.GetPlayerPawn` 0) 5.0 true)
    (else
      (set `self.IsSeeingPlayer?` false))))

(fn `UserConstructionScript`)