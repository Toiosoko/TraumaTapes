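; BP_EnemyController is the enemy AI controller that starts the BT_EnemyIA behavior tree.
; On BeginPlay it caches the player character, then runs the tree after a short delay.
; UpdateNearDoor stores the door proximity flag and passes door state to the blackboard.
; Its IsDoorLocked input is written unchanged to the IsDoorOpen key, so name and key differ in meaning.
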(event `self.ReceiveBeginPlay`
  (set `self.PlayerReference` (`GameplayStatics.GetPlayerCharacter` 0))
  (`KismetSystemLibrary.Delay` 0.2)
  (`self.RunBehaviorTree` "/Game/LoryTest/Blueprints/BT_EnemyIA.BT_EnemyIA"))

(event `/Game/LoryTest/Blueprints/Interface/IF_DoorNear.Update Near Door`
  (params (NearDoor :type Boolean) (IsDoorLocked :type Boolean))
  (bind _blackboard (`self.Blackboard`))
  ;[1 1 1] Near Door Update
  (bind _output_get (set `self.NearDoor` NearDoor))
  (`BlackboardComponent.SetValueAsBool` _blackboard "NearDoor" _output_get)
  (`BlackboardComponent.SetValueAsBool` _blackboard "IsDoorOpen" IsDoorLocked))

(fn `UserConstructionScript`)