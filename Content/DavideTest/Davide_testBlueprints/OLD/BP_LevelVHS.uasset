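; BP_LevelVHS is an actor representing a VHS tape tied to a level, kept in a test OLD folder.
; On BeginPlay it copies the tape name, level name and level object from its VHSData into its own variables.
; The IsPlayable copy is never executed, and the Blueprint has no logic for interacting with the tape or loading the level.
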(event `self.ReceiveBeginPlay`
  (bind _vhs_data_0 (`self.VHS Data_0`))
  (set `self.VHS Name_0` (`/Game/DavideTest/Davide_testBlueprints/VHS_DataAssets/PDA_VHS_Structure.VHS Name` _vhs_data_0))
  (set `self.LevelPlayed_0` (`/Game/DavideTest/Davide_testBlueprints/VHS_DataAssets/PDA_VHS_Structure.LevelPlayedName` _vhs_data_0))
  (set `self.LevelPlayed Object_0` (`/Game/DavideTest/Davide_testBlueprints/VHS_DataAssets/PDA_VHS_Structure.LevelPlayedObject` _vhs_data_0)))

(fn `UserConstructionScript`
  (`parent.UserConstructionScript`))